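; BP_Patroller is an enemy AI pawn that patrols between targets in its TargetList, starting on BeginPlay.
; MoveNPC picks a list entry and uses AIMoveTo toward a reachable point close around it.
; It calls itself after a pause on success or a brief retry delay on failure, stopping if the target is invalid.
; The random index has Min and Max reversed, so it resolves to the last entry.
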(event Custom|MoveNPC
  (bind _targetlist (Variables|Default|GetTargetList))
  (bind _output_get (Variables|Default|SetCurrentTarget (Utilities|Array|Get(acopy) _targetlist (Math|Random|RandomIntegerinRange (Utilities|Array|LastIndex _targetlist) 0))))
  (Utilities|IsValid _output_get
    (:Is%20Valid
      (bind _output_get_2 (Variables|Default|SetRandom%20Location (.RandomLocation (AI|Navigation|GetRandomReachablePointinRadius (Transformation|GetActorLocation (Variables|Default|GetCurrentTarget)) 5.0 0 0))))
      (AI|AIMoveTo self _output_get_2 0 5.0 false
        (:OnSuccess
          (Utilities|FlowControl|Delay 2.0)
          (CallFunction|MoveNPC))
        (:OnFail
          (Utilities|FlowControl|Delay 0.1)
          (CallFunction|MoveNPC))))))

(event EventBeginPlay
  (CallFunction|MoveNPC))

(fn ConstructionScript)